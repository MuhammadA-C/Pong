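; Player controller for a paddle game that owns the HUD and moves the player's paddle pawn with W and S.
; Key presses set movement flags that Tick reads, shifting the paddle along X with a swept SetActorLocation by its Speed per frame, unscaled by delta time.
; BeginPlay creates the HUD and binds to its game-over dispatcher, which leads to disabling input and showing the mouse cursor.
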(event `self.ReceiveBeginPlay`
  (bind _returnvalue (`|CreateWidget` "/Game/Blueprints/UI/WBP_Hud.WBP_Hud_C"))
  (bind _output_get (set `self.Hud` _returnvalue))
  (`UserWidget.AddToViewport` _output_get 0)
  (add `/Game/Blueprints/UI/WBP_Hud.GameOver_ED` _output_get (delegate `GameOver_ED_Event`)))

(event `GameOver_ED_Event`
  (`self.GameOver_Event`))

(event `Key|W`
  (params (Key :type "Key Structure"))
  ;[1 1 1] Player Controls
  (:`Pressed`
    (set `self.bIsMovingUp` true))
  (:`Released`
    (set `self.bIsMovingUp` false)))

(event `Key|S`
  (params (Key :type "Key Structure"))
  ;[1 1 1] Player Controls
  (:`Pressed`
    (set `self.bIsMovingDown` true))
  (:`Released`
    (set `self.bIsMovingDown` false)))

(event `self.ReceiveTick`
  (params (DeltaSeconds :type "Float (single-precision)"))
  ;[1 1 1] Paddle Movement
  (`|ExecutionSequence`
    (:`then_0`
      (if (`self.bIsMovingUp`)
        (`self.MovePaddleUp`)))
    (:`then_1`
      (if (`self.bIsMovingDown`)
        (`self.MovePaddleDown`)))))

(event `GameOver_Event`
  ;[1 1 1] Game Over
  (`self.DisableInput` null)
  (set `self.bShowMouseCursor` true))

(fn `UserConstructionScript`)