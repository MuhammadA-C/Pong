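; BP_AIPaddle is the AI-controlled paddle that tracks the ball along the X axis.
; On BeginPlay it calls StartGame on BP_GameState, takes its Balls list and binds to the first ball's destroyed dispatcher.
; Each Tick it makes a swept move to the first ball's X, keeping its own Y and Z.
; Ball destruction sets a never-reset flag that switches Tick from following to removing the list's first entry.
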(event `self.ReceiveBeginPlay`
  ;[1 1 1] Gets a reference to the ball at the start of the game so the AI paddle can follow its movement
  (bind _asbp_game_state (cast `/Game/Blueprints/GameMode/BP_GameState` (`GameplayStatics.GetGameState`)))
  (`/Game/Blueprints/GameMode/BP_GameState.StartGame` _asbp_game_state)
  (bind _balls (`/Game/Blueprints/GameMode/BP_GameState.Balls` _asbp_game_state))
  (set `self.ListOfBalls` _balls)
  ;[1 1 1] Used to detect when the ball is destroyed to remove it from the array
  (add `/Game/Blueprints/BP_Ball.Destroyed_EventDispatcher` (`|GetArrayItem` _balls) (delegate `Destroyed_EventDispatcher_Event`)))

(event `Destroyed_EventDispatcher_Event`
  ;[1 1 1] Used to detect when the ball is destroyed to remove it from the array
  (set `self.bRemoveBall` true))

(event `self.ReceiveTick`
  (params (DeltaSeconds :type "Float (single-precision)"))
  (if (`self.bRemoveBall`)
    ;[1 0.5732 0.1969] NOTE: In the future might need to add a call to reset "RemoveBall" to false, and add a length check on the array prioro to calling "Follow Ball"
    (`KismetArrayLibrary.Array_Remove` (`self.ListOfBalls`)) ; Have to remove the ball from the array when it's destroyed so we don't access
    (else
      (`self.FollowBall`))))

(fn `UserConstructionScript`)