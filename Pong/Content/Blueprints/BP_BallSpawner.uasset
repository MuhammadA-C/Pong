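; BP_BallSpawner is an actor that spawns a BP_Ball at its own transform to start the game and each following round.
; It spawns one ball on BeginPlay and binds to the StartNextRound dispatcher on BP_GameMode.
; When that dispatcher fires, StartRound waits a short delay and then spawns a new ball.
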(event `self.ReceiveBeginPlay`
  (`|ExecutionSequence`
    (:`then_0`
      ;[1 1 1] Comment
      (bind _asbp_game_mode (cast `/Game/Blueprints/GameMode/BP_GameMode` (`GameplayStatics.GetGameMode`)))
      (add `/Game/Blueprints/GameMode/BP_GameMode.StartNextRound` _asbp_game_mode (delegate `StartNextRound_Event`)))
    (:`then_1`
      ;[1 1 1] Spawns ball at start of game
      (`|SpawnActorFromClass` "/Game/Blueprints/BP_Ball.BP_Ball_C" (`self.GetTransform`) "Undefined" "MultiplyWithRoot" null null))))

(event `StartNextRound_Event`
  ;[1 1 1] Comment
  (`self.StartRound`))

(event `StartRound`
  ;[1 1 1] Starts the next round
  (`KismetSystemLibrary.Delay` 2.0)
  (`|SpawnActorFromClass` "/Game/Blueprints/BP_Ball.BP_Ball_C" (`self.GetTransform`) "Undefined" "MultiplyWithRoot" null null))

(fn `UserConstructionScript`)