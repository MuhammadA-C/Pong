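; Game state Blueprint that tracks scores and drives round flow in a ball game.
; On BeginPlay it gathers the tagged ball actors and caches BP_GameMode.
; UpdateScore overwrites the score of an existing player key and broadcasts ScoresUpdated.
; It then asks the game mode whether the win condition is met, triggering GameOver with the winner or broadcasting NextRound.
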(event `self.ReceiveBeginPlay`
  (`self.StartGame`)
  (bind _asbp_game_mode (cast `/Game/Blueprints/GameMode/BP_GameMode` (`GameplayStatics.GetGameMode`)))
  (set `self.GameMode` _asbp_game_mode))

(event `StartGame`
  ;[1 1 1] Gets a reference to the ball
  (bind _outactors (`GameplayStatics.GetAllActorsOfClassWithTag` "/Game/Blueprints/BP_Ball.BP_Ball_C" "Ball"))
  (set `self.Balls` _outactors))

(event `UpdateScore`
  (params (PlayerKey :type String) (UpdateValue :type Integer))
  (bind _scores (`self.Scores`))
  ;[1 1 1] Updates Score
  (`|ExecutionSequence`
    (:`then_0`
      (if (`BlueprintMapLibrary.Map_Contains` _scores PlayerKey)
        (`BlueprintMapLibrary.Map_Add` _scores PlayerKey UpdateValue)
        (`self.ScoresUpdated`)))
    (:`then_1`
      ;[1 1 1] Checks if the game is over or continue to the next round
      (bind (_waswinconditionmet _winner) (`/Game/Blueprints/GameMode/BP_GameMode.WasWinConditionMet` (`self.GameMode`) (`self.Scores`)))
      (if _waswinconditionmet
        (`/Game/Blueprints/GameMode/BP_GameMode.GameOver` (`self.GameMode`) _winner)
        (else
          (`self.NextRound`))))))

(fn `UserConstructionScript`)