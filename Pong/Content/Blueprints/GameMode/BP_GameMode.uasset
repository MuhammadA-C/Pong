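; Game mode Blueprint that defines the score-based win check and handles game over and restart.
; WasWinConditionMet loops over the keys of a Scores map and stops at the first score exactly equal to MaxScore, returning a flag and that key as the winner.
; GameOver_Event only stores the winner, and RestartGame_Event calls RestartGame.
; Ties are not handled.
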(event `GameOver_Event`
  (params (Winner :type String))
  ;[1 1 1] Game Over
  (set `self.Winner` Winner))

(event `RestartGame_Event`
  ;[1 1 1] Restarts Game
  (`self.RestartGame`))

(fn `UserConstructionScript`)

(fn `WasWinConditionMet`
  (params (Scores :type "Map of String to Integer"))
  (returns (WasWinConditionMet :type Boolean) (Winner :type String))
  (locals (bMetWinCondition :type Boolean) (WinnersName :type String))
  ;[1 0.5691 0.2001] NOTE: We might want to add a length check to ensure the array isn't empty
  (bind _keys (`BlueprintMapLibrary.Map_Keys` Scores))
  (for _array_element _keys
    ;[1 0.5454 0.1629] NOTE: This section of the code will need to be fixed to account for ties in the future if we want ties because currently it doesn't
    (if (== (`BlueprintMapLibrary.Map_Find` Scores _array_element) (`self.MaxScore`))
      (set `local.bMetWinCondition` true)
      (set `local.WinnersName` _array_element)
      (break)))
  (return (`local.bMetWinCondition`) (`local.WinnersName`)))