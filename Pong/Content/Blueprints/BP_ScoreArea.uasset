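; BP_ScoreArea is a goal trigger that awards a point when a BP_Ball enters its box.
; On overlap it destroys the ball, then looks up its PlayerKey in the Scores map on BP_GameState.
; If the key exists, it increments that value and passes it to the game state's UpdateScore.
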(event `self.Box.OnComponentBeginOverlap`
  (params (OverlappedComponent :type "PrimitiveComponent Object Reference") (OtherActor :type "Actor Object Reference") (OtherComp :type "PrimitiveComponent Object Reference") (OtherBodyIndex :type Integer) (bFromSweep :type Boolean) (SweepResult :type "HitResult Structure (by ref)"))
  (bind _asbp_ball (cast `/Game/Blueprints/BP_Ball` OtherActor))
  (`/Game/Blueprints/BP_Ball.DestroyBall` _asbp_ball)
  (bind _asbp_game_state (cast `/Game/Blueprints/GameMode/BP_GameState` (`GameplayStatics.GetGameState`)))
  (bind (_value _returnvalue) (`BlueprintMapLibrary.Map_Find` (`/Game/Blueprints/GameMode/BP_GameState.Scores` _asbp_game_state) (`self.PlayerKey`)))
  (if _returnvalue
    (bind _result (`/Engine/EditorBlueprintResources/StandardMacros.IncrementInt` _value)
      (:`  `
        (`/Game/Blueprints/GameMode/BP_GameState.UpdateScore` _asbp_game_state (`self.PlayerKey`) _result)))))

(fn `UserConstructionScript`)