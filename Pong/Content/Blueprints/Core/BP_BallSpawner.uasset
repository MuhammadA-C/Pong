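; BP_BallSpawner is an actor that spawns the game's BP_Ball at its own transform at game start and each new round.
; On BeginPlay it caches the BP_GameState, binds to the BP_GameMode's StartNextRound dispatcher and spawns the first ball.
; When that dispatcher fires, StartRound spawns another ball and calls StartGame on the game state, which the initial spawn does not do.
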(event `self.ReceiveBeginPlay`
  (`|ExecutionSequence`
    (:`then_0`
      (bind _asbp_game_state (cast `/Game/Blueprints/GameMode/BP_GameState` (`GameplayStatics.GetGameState`)))
      (set `self.As BP Game State` _asbp_game_state))
    (:`then_1`
      ;[1 1 1] Comment
      (bind _asbp_game_mode (cast `/Game/Blueprints/GameMode/BP_GameMode` (`GameplayStatics.GetGameMode`)))
      (add `/Game/Blueprints/GameMode/BP_GameMode.StartNextRound` _asbp_game_mode (delegate `StartNextRound_Event`)))
    (:`then_2`
      ;[1 1 1] Spawns ball at start of game
      (`|SpawnActorFromClass` "/Game/Blueprints/Core/BP_Ball.BP_Ball_C" (`self.GetTransform`) "Undefined" "MultiplyWithRoot" null null))))

(event `StartNextRound_Event`
  ;[1 1 1] Comment
  (`self.StartRound`))

(event `StartRound`
  ;[1 1 1] Starts the next round
  (`|SpawnActorFromClass` "/Game/Blueprints/Core/BP_Ball.BP_Ball_C" (`self.GetTransform`) "Undefined" "MultiplyWithRoot" null null)
  (`/Game/Blueprints/GameMode/BP_GameState.StartGame` (`self.As BP Game State`)))

(fn `UserConstructionScript`)