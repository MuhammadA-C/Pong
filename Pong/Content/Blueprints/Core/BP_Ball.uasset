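; Physics-driven ball actor that launches along Y at BeginPlay and bounces off actors tagged Paddle or Wall.
; On a hit, the IsMovingForward macro samples the sphere's Y position across a short Delay to pick the sign of a Y force applied at the impact point.
; The Destroy event removes the Ball tag, destroys the actor and calls a destroyed event dispatcher.
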(event `self.ReceiveBeginPlay`
  ;[1 1 1] Pushes the ball at the start of the game
  (`PrimitiveComponent.AddForce` (`self.Sphere`) (0.0 100000.0 0.0) "None" true))

(event `self.Sphere.OnComponentHit`
  (params (HitComponent :type "PrimitiveComponent Object Reference") (OtherActor :type "Actor Object Reference") (OtherComp :type "PrimitiveComponent Object Reference") (NormalImpulse :type "Vector Structure") (Hit :type "HitResult Structure (by ref)"))
  (bind _sphere (`self.Sphere`))
  ;[1 1 1] Adds an opposite force when the ball hits a wall or paddle to make to the ball bounce back
  (if (or (`self.ActorHasTag` OtherActor "Paddle") (`self.ActorHasTag` OtherActor "Wall"))
    (`self.IsMovingForward`
      (:`yes`
        (`PrimitiveComponent.AddForceAtLocation` _sphere (0.0 -100000.0 0.0) Hit_ImpactPoint "None"))
      (:`no`
        (`PrimitiveComponent.AddForceAtLocation` _sphere (0.0 100000.0 0.0) Hit_ImpactPoint "None")))))

(event `DestroyBall`)

(event `/Game/Blueprints/Interfaces/BPI_Destroyed.Destroy`
  (`KismetArrayLibrary.Array_RemoveItem` (`self.ActorTags`) "Ball")
  (`self.K2_DestroyActor`)
  (`self.Destroyed_EventDispatcher`))

(fn `UserConstructionScript`
  ;[1 1 1] Adds actor tag
  (set `self.Tags` (`self.ActorTags`)))